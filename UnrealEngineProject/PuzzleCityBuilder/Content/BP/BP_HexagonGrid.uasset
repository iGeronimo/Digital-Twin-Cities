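; BP_HexagonGrid generates a hexagon-shaped grid of BP_HexagonTile actors at BeginPlay and attaches them to itself.
; TransformCalculation derives spacing from the scaled mesh bounds, builds rows up to the middle, then mirrors all but the middle across X.
; After the spawn loop, only the last tile's mesh components reach BP_BuildManager and only it gets a coordinate ID.
; An instanced mesh component is still created, but its instancing call never runs.
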(event EventBeginPlay
  (bind _gridmeshsize (Variables|Default|GetgridMeshSize))
  (bind (_x _y) (Math|Vector|BreakVector _gridmeshsize))
  (CallFunction|TransformCalculation)
  (for _array_element (Variables|Default|GetgridTransforms)
    (bind _returnvalue (Game|SpawnActorfromClass "/Game/BP/BP_HexagonTile.BP_HexagonTile_C" _array_element "Undefined" "MultiplyWithRoot" 0 0))
    (Transformation|AttachActorToActor _returnvalue self "None" "KeepRelative" "KeepRelative" "KeepRelative" true))
  (bind _returnvalue_2 (Actor|GetActorOfClass "/Game/BP/BP_BuildManager.BP_BuildManager_C"))
  (Variables|/Game/BP/BP_BuildManager.BP_BuildManager_C|SetTileComponents _returnvalue_2 (Actor|GetComponentsByClass _returnvalue "/Script/Engine.StaticMeshComponent"))
  (Variables|/Game/BP/BP_HexagonTile.BP_HexagonTile_C|SetTileCoordID _returnvalue (Math|Vector2D|MakeVector2D (Math|Conversions|ToFloat(Integer) (Math|Float|Round (Utilities|Operators|Divide (.Y (Math|Vector|BreakVector (.Location (Math|Transform|BreakTransform _array_element)))) _y 0.9))) (Math|Conversions|ToFloat(Integer) (Math|Float|Round (Utilities|Operators|Divide (.X (Math|Vector|BreakVector (.Location (Math|Transform|BreakTransform _array_element)))) _x 0.9))))))

(event Collision|EventActorBeginOverlap
  (params (OtherActor :type Actor%20Object%20Reference)))

(event EventTick
  (params (DeltaSeconds :type Float%20%28single-precision%29)))

(fn ConstructionScript)

(fn TransformCalculation
  (bind _inputgridmesh (Variables|Default|GetinputGridMesh))
  (bind _returnvalue (StaticMesh|GetBoundingBox _inputgridmesh))
  (bind (_min _max) (Utilities|Struct|BreakBox _returnvalue))
  (Variables|Default|SetgridRadiusAdjusted (- (Variables|Default|GetgridRadius) 1))
  (Variables|Default|SetgridMeshSize (* (- _max _min) (Variables|Default|GetgridMeshScale)))
  (bind _returnvalue_2 (AddComponent|AddInstancedStaticMeshComponent false))
  (bind _output_get (Variables|Default|SetISM_gridMesh _returnvalue_2))
  (Components|StaticMesh|SetStaticMesh _output_get (Variables|Default|GetinputGridMesh))
  (Utilities|FlowControl|Sequence
    (:then_0
      ;[1 1 1] Transform calculation
      (for _index (range 0 (Variables|Default|GetgridRadiusAdjusted))
        (for _index_2 (range 0 (+ _index (Variables|Default|GetgridRadiusAdjusted)))
          (Utilities|Array|Add (Variables|Default|GetgridTransforms) (Math|Transform|MakeTransform (Math|Vector|MakeVector (* (Math|Conversions|ToFloat(Integer) (- _index (Variables|Default|GetgridRadiusAdjusted))) (- (.X (Math|Vector|BreakVector (Variables|Default|GetgridMeshSize))) (* (.X (Math|Vector|BreakVector (Variables|Default|GetgridMeshSize))) 0.25))) (- (/ (* (.Y (Math|Vector|BreakVector (Variables|Default|GetgridMeshSize))) (Math|Conversions|ToFloat(Integer) (+ _index (Variables|Default|GetgridRadiusAdjusted)))) 2.0) (* (.Y (Math|Vector|BreakVector (Variables|Default|GetgridMeshSize))) (Math|Conversions|ToFloat(Integer) _index_2))) 0.0) "0, 0, 0" (Math|Conversions|ToVector(Float) (Variables|Default|GetgridMeshScale)))))))
    (:then_1
      (for (_array_element _array_index) (Variables|Default|GetgridTransforms)
        (if (< _array_index (Utilities|Operators|Subtract (Utilities|Array|Length (Variables|Default|GetgridTransforms)) (Variables|Default|GetgridRadius) (Variables|Default|GetgridRadiusAdjusted)))
          (Utilities|Array|Add (Variables|Default|GetgridNewTransforms) (Math|Transform|MakeTransform (* (.Location (Math|Transform|BreakTransform _array_element)) "-1.000000,1.000000,1.000000") (.Rotation (Math|Transform|BreakTransform _array_element)) (.Scale (Math|Transform|BreakTransform _array_element)))))))
    (:then_2
      (Utilities|Array|AppendArray (Variables|Default|GetgridTransforms) (Variables|Default|GetgridNewTransforms)))))
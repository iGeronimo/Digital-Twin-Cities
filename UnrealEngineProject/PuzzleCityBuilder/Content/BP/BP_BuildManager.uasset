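; BP_BuildManager is an input-driven selector for the type of building or tile currently chosen in a build system.
; On BeginPlay it finds the PlayerController actors and enables click events on the first one.
; Releasing Z, X, C, V, B or N sets CurrentTileType to one of six enum values, then a shared print reports the selection on screen.
; Placement logic is not in this Blueprint.
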(event EventBeginPlay
  (bind _outactors (Actor|GetAllActorsOfClass "/Script/Engine.PlayerController"))
  (Variables|/Script/Engine.PlayerController|SetbEnableClickEvents (Utilities|Array|Get(acopy) _outactors) true))

(event Input|KeyboardEvents|Z
  (params (Key :type Key%20Structure :default "None"))
  (:Released
    (Variables|Default|SetCurrentTileType "NewEnumerator0")
    (Development|PrintString (Utilities|String|Append (Utilities|String|MakeLiteralString "Current Building Seleceted: ") (Utilities|String|EnumtoString (Variables|Default|GetCurrentTileType))))))

(event Input|KeyboardEvents|X
  (params (Key :type Key%20Structure :default "None"))
  (:Released
    (Variables|Default|SetCurrentTileType "NewEnumerator1")
    (Development|PrintString (Utilities|String|Append (Utilities|String|MakeLiteralString "Current Building Seleceted: ") (Utilities|String|EnumtoString (Variables|Default|GetCurrentTileType))))))

(event Input|KeyboardEvents|C
  (params (Key :type Key%20Structure :default "None"))
  (:Released
    (Variables|Default|SetCurrentTileType "NewEnumerator2")
    (Development|PrintString (Utilities|String|Append (Utilities|String|MakeLiteralString "Current Building Seleceted: ") (Utilities|String|EnumtoString (Variables|Default|GetCurrentTileType))))))

(event Input|KeyboardEvents|V
  (params (Key :type Key%20Structure :default "None"))
  (:Released
    (Variables|Default|SetCurrentTileType "NewEnumerator3")
    (Development|PrintString (Utilities|String|Append (Utilities|String|MakeLiteralString "Current Building Seleceted: ") (Utilities|String|EnumtoString (Variables|Default|GetCurrentTileType))))))

(event Input|KeyboardEvents|B
  (params (Key :type Key%20Structure :default "None"))
  (:Released
    (Variables|Default|SetCurrentTileType "NewEnumerator4")
    (Development|PrintString (Utilities|String|Append (Utilities|String|MakeLiteralString "Current Building Seleceted: ") (Utilities|String|EnumtoString (Variables|Default|GetCurrentTileType))))))

(event Input|KeyboardEvents|N
  (params (Key :type Key%20Structure :default "None"))
  (:Released
    (Variables|Default|SetCurrentTileType "NewEnumerator5")
    (Development|PrintString (Utilities|String|Append (Utilities|String|MakeLiteralString "Current Building Seleceted: ") (Utilities|String|EnumtoString (Variables|Default|GetCurrentTileType))))))

(fn ConstructionScript)
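; BP_Telemetry records playtest session telemetry, toggled on and off with the T key.
; Starting stores the time and BP_NecessityManager score and writes a tile-change header; tile entries are not added in this graph.
; While active, left and right mouse presses share one counter, which is never reset here.
; Stopping appends clicks, duration and scores, exports to a text file unless overwriting is disallowed, then clears the data.
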(event EventBeginPlay)

(event Collision|EventActorBeginOverlap
  (params (OtherActor :type Actor%20Object%20Reference)))

(event EventTick
  (params (DeltaSeconds :type Float%20%28single-precision%29)))

(event Input|KeyboardEvents|T
  (params (Key :type Key%20Structure :default "None"))
  (bind _telemetrydata (Variables|Default|GetTelemetryData))
  (:Pressed
    (Variables|Default|SetTelemetryInProcess (not (Variables|Default|GetTelemetryInProcess)))
    (if (Variables|Default|GetTelemetryInProcess)
      (Development|PrintString "Telemetry started")
      (Variables|Default|SetStartingTime (Math|DateTime|Now))
      (Utilities|Array|Add (Variables|Default|GetTelemetryData) "Tile changes during session. The data is shown as \"Tile coordinates; Old tile state; New tile state; Time at which it was changed\":")
      (bind _returnvalue (Actor|GetActorOfClass "/Game/BP/BP_NecessityManager.BP_NecessityManager_C"))
      (Variables|Default|SetStartingScore (Variables|/Game/BP/BP_NecessityManager.BP_NecessityManager_C|GetScore _returnvalue))
      (else
        (Development|PrintString "Telemetry finished")
        (Utilities|Array|Add _telemetrydata "")
        (Utilities|Array|Add _telemetrydata (Utilities|String|Append "Number of times left and right mouse button was pressed: " (Utilities|String|ToString(Integer) (Variables|Default|GetNumMouseClicks))))
        (Utilities|Array|Add _telemetrydata (Utilities|String|Append "Time spent in session in seconds: " (Utilities|String|ToString(Integer) (.OutputMinutes (CallFunction|ConvertTimeSpantoSeconds (- (Math|DateTime|Now) (Variables|Default|GetStartingTime))))) "m " (Utilities|String|ToString(Integer) (.OutputSeconds (CallFunction|ConvertTimeSpantoSeconds (- (Math|DateTime|Now) (Variables|Default|GetStartingTime))))) "s"))
        (Utilities|Array|Add (Variables|Default|GetTelemetryData) (Utilities|String|Append "Score at the start of the session: " (Utilities|String|ToString(Integer) (Variables|Default|GetStartingScore))))
        (Utilities|Array|Add (Variables|Default|GetTelemetryData) (Utilities|String|Append "Score at the end of the session: " (Utilities|String|ToString(Integer) (Variables|/Game/BP/BP_NecessityManager.BP_NecessityManager_C|GetScore _returnvalue))))
        (if (Class|BlueprintPathsLibrary|FileExists (Utilities|String|Append (Utilities|Struct|BreakDirectoryPath (Variables|Default|GetExportPath)) "/" (Variables|Default|GetFileName) ".txt"))
          (if (Variables|Default|GetOverwriteFile)
            (Class|TelemetryDataExport|ExportTelemetryData (Variables|Default|GetTelemetryData) (Variables|Default|GetFileName) (Variables|Default|GetExportPath) :!label _label)
            (Utilities|Array|Clear (Variables|Default|GetTelemetryData))
            (else
              (Development|PrintString "File exists already. Enable file overwrite if you would like to overwrite file.")
              (Utilities|Array|Clear (Variables|Default|GetTelemetryData))))
          (else
            (goto _label)))))))

(event Input|MouseEvents|LeftMouseButton
  (params (Key :type Key%20Structure :default "None"))
  (:Pressed
    (if (Variables|Default|GetTelemetryInProcess)
      (Math|Integer|IncrementInt (Variables|Default|GetNumMouseClicks)))))

(event Input|MouseEvents|RightMouseButton
  (params (Key :type Key%20Structure :default "None"))
  (:Pressed
    (if (Variables|Default|GetTelemetryInProcess)
      (Math|Integer|IncrementInt (Variables|Default|GetNumMouseClicks)))))

(fn ConstructionScript)

(fn ConvertTimeSpantoSeconds
  (params (InputValue :type Timespan%20Structure))
  (bind (_days _hours _minutes _seconds _milliseconds) (Math|Timespan|BreakTimespan InputValue))
  (bind _returnvalue (Math|Float|MakeLiteralFloat 0.001))
  (bind _returnvalue_2 (* _days 86400))
  (bind _returnvalue_3 (* _hours 3600))
  (bind _returnvalue_4 (* _minutes 60))
  (bind _returnvalue_5 (* _milliseconds _returnvalue))
  (bind _returnvalue_6 (Math|Float|Round _returnvalue_5))
  (bind _returnvalue_7 (+ _returnvalue_2 _returnvalue_3 _returnvalue_4 _seconds _returnvalue_6))
  (bind _returnvalue_8 (Math|Conversions|ToFloat(Integer) _returnvalue_7))
  (bind (_remainder _returnvalue_9) (Math|Float|Division(WholeandRemainder) _returnvalue_8 6e+01))
  (return _returnvalue_9 (Math|Float|Round _remainder)))
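; Top-down style camera pawn for the hex grid map that handles panning and zooming, and creates the build-buttons HUD on BeginPlay.
; Tick moves CameraHolder by WASD or left-mouse drag, rotated to its starting yaw and not scaled by delta time.
; The mouse wheel slides the Camera along local X for zoom.
; Tick clamps zoom and limits panning to bounds derived from BP_HexagonGrid's radius around the start position.
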(event EventBeginPlay
  (bind _cameraholder (Variables|Default|GetCameraHolder))
  (Variables|/Script/Engine.PlayerController|SetbShowMouseCursor (Game|GetPlayerController (Game|GetPlayerState 0)) true)
  (Variables|Default|SetCameraStartingWorldPosition (Transformation|GetWorldLocation _cameraholder))
  (Variables|Default|SetCameraStartingRelativePosition (CallFunction|GetRelativeLocation _cameraholder))
  (Variables|Default|SetCameraRotatorZ (Math|Rotator|MakeRotator 0.0 0.0 (.Yaw (Math|Rotator|BreakRotator (Transformation|GetWorldRotation (Variables|Default|GetCameraHolder))))))
  (bind _returnvalue (Actor|GetActorOfClass "/Game/BP/BP_HexagonGrid.BP_HexagonGrid_C"))
  (Variables|Default|SetCameraPanLimit (Math|Vector2D|MakeVector2D (Math|Conversions|ToFloat(Integer) (* (Variables|/Game/BP/BP_HexagonGrid.BP_HexagonGrid_C|GetgridRadius _returnvalue) 1000)) (Math|Conversions|ToFloat(Integer) (* (Variables|/Game/BP/BP_HexagonGrid.BP_HexagonGrid_C|GetgridRadius _returnvalue) 1000))))
  (bind _returnvalue_2 (UserInterface|CreateWidget "/Game/BP/BP_UIBuildButtons.BP_UIBuildButtons_C" (Game|GetPlayerController 0)))
  (bind _output_get (Variables|Default|SetBuildingHUD _returnvalue_2))
  (UserInterface|Viewport|AddtoViewport _output_get 0))

(event EventTick
  (params (DeltaSeconds :type Float%20%28single-precision%29))
  (bind _camerapanlimit (Variables|Default|GetCameraPanLimit))
  (bind _camera (Variables|Default|GetCamera))
  (bind _camerastartingworldposition (Variables|Default|GetCameraStartingWorldPosition))
  (bind _camerazoomlimit (Variables|Default|GetCameraZoomLimit))
  (bind _cameraholder (Variables|Default|GetCameraHolder))
  (bind _cameraholder_2 (Variables|Default|GetCameraHolder))
  (bind _cameraholder_3 (Variables|Default|GetCameraHolder))
  (bind _returnvalue (Transformation|GetWorldLocation _cameraholder_2))
  (bind _returnvalue_2 (Transformation|GetWorldLocation _cameraholder_3))
  (bind (_x _y) (Math|Vector|BreakVector _camerastartingworldposition))
  (bind (_x_2 _y_2) (Math|Vector2D|BreakVector2D _camerapanlimit))
  (bind _return_value (CallFunction|GetRelativeLocation _camera))
  (bind (_x_3 _y_3 _z) (Math|Vector|BreakVector _returnvalue))
  (bind (_x_4 _y_4 _z_2) (Math|Vector|BreakVector _returnvalue_2))
  (bind (_x_5 _y_5 _z_3) (Math|Vector|BreakVector _return_value))
  (Utilities|FlowControl|Sequence
    (:then_0
      ;[1 1 1] WASD Camera Position Control
      (Transformation|SetWorldLocation _cameraholder (+ (Transformation|GetWorldLocation _cameraholder) (* (Variables|Default|GetCameraPanKeyboardSpeed) (Math|Vector|RotateVector (Variables|Default|GetCameraPanDirection) (Variables|Default|GetCameraRotatorZ)))) false false))
    (:then_1
      ;[1 1 1] Mouse Camera Position Control
      (if (Variables|Default|GetLMBDown)
        (if (Utilities|Operators|EqualEqual :A (Variables|Default|GetMousePositionStored))
          _
          (else
            (bind _returnvalue_3 (Class|WidgetLayoutLibrary|GetMousePositiononViewport))
            (Transformation|SetWorldLocation (Variables|Default|GetCameraHolder) (Math|Vector|MakeVector (+ _x_3 (.Y (Math|Vector|BreakVector (* (Math|Vector|RotateVector (Math|Conversions|ToVector(Vector2D) (- _returnvalue_3 (Variables|Default|GetMousePositionStored))) (Variables|Default|GetCameraRotatorZ)) (Variables|Default|GetCameraPanMouseSpeed))))) (- _y_3 (.X (Math|Vector|BreakVector (* (Math|Vector|RotateVector (Math|Conversions|ToVector(Vector2D) (- _returnvalue_3 (Variables|Default|GetMousePositionStored))) (Variables|Default|GetCameraRotatorZ)) (Variables|Default|GetCameraPanMouseSpeed))))) _z) false false)))
        (bind _returnvalue_4 (Class|WidgetLayoutLibrary|GetMousePositiononViewport))
        (Variables|Default|SetMousePositionStored _returnvalue_4)
        (else
          (Variables|Default|SetMousePositionStored ""))))
    (:then_2
      ;[1 1 1] Camera Limit Control
      (Utilities|FlowControl|Sequence
        (:then_0
          (Transformation|SetWorldLocation (Variables|Default|GetCameraHolder) (Math|Vector|MakeVector (Math|Float|Min(Float) (Math|Float|Max(Float) _x_4 (- _x _y_2)) (+ _x _y_2)) (Math|Float|Min(Float) (Math|Float|Max(Float) _y_4 (- _y _x_2)) (+ _y _x_2)) _z_2) false false))
        (:then_1
          (Transformation|SetRelativeLocation (Variables|Default|GetCamera) (Math|Vector|MakeVector (Math|Float|Min(Float) (Math|Float|Max(Float) _x_5 (* _camerazoomlimit -1.0)) _camerazoomlimit) _y_5 _z_3) false false))))))

(event Input|MouseEvents|MouseWheelAxis
  (params (AxisValue :type Float%20%28single-precision%29))
  (bind _camera (Variables|Default|GetCamera))
  (bind _return_value (CallFunction|GetRelativeLocation _camera))
  (bind (_x _y _z) (Math|Vector|BreakVector _return_value))
  ;[1 1 1] Mouse Wheel Camera Zoom Control
  (Transformation|SetRelativeLocation (Variables|Default|GetCamera) (Math|Vector|MakeVector (+ (* AxisValue (Variables|Default|GetCameraZoomSpeed)) _x) _y _z) false false))

(event Input|KeyboardEvents|D
  (params (Key :type Key%20Structure :default "None"))
  ;[1 1 1] WASD Camera Direction Control
  (:Pressed
    (Variables|Default|SetCameraPanDirection (+ (Variables|Default|GetCameraPanDirection) "0.000000,1.000000,0.000000")))
  (:Released
    (Variables|Default|SetCameraPanDirection (- (Variables|Default|GetCameraPanDirection) "0.000000,1.000000,0.000000"))))

(event Input|KeyboardEvents|A
  (params (Key :type Key%20Structure :default "None"))
  ;[1 1 1] WASD Camera Direction Control
  (:Pressed
    (Variables|Default|SetCameraPanDirection (+ (Variables|Default|GetCameraPanDirection) "0.000000,-1.000000,0.000000")))
  (:Released
    (Variables|Default|SetCameraPanDirection (- (Variables|Default|GetCameraPanDirection) "0.000000,-1.000000,0.000000"))))

(event Input|KeyboardEvents|W
  (params (Key :type Key%20Structure :default "None"))
  ;[1 1 1] WASD Camera Direction Control
  (:Pressed
    (Variables|Default|SetCameraPanDirection (+ (Variables|Default|GetCameraPanDirection) "1.000000,0.000000,0.000000")))
  (:Released
    (Variables|Default|SetCameraPanDirection (- (Variables|Default|GetCameraPanDirection) "1.000000,0.000000,0.000000"))))

(event Input|KeyboardEvents|S
  (params (Key :type Key%20Structure :default "None"))
  ;[1 1 1] WASD Camera Direction Control
  (:Pressed
    (Variables|Default|SetCameraPanDirection (+ (Variables|Default|GetCameraPanDirection) "-1.000000,0.000000,0.000000")))
  (:Released
    (Variables|Default|SetCameraPanDirection (- (Variables|Default|GetCameraPanDirection) "-1.000000,0.000000,0.000000"))))

(event Input|MouseEvents|LeftMouseButton
  (params (Key :type Key%20Structure :default "None"))
  ;[1 1 1] Mouse Press Down Camera Control
  (:Pressed
    (Variables|Default|SetLMBDown true))
  (:Released
    (Variables|Default|SetLMBDown false)))

(fn ConstructionScript)

(fn GetRelativeLocation
  (params (Target :type Scene%20Component%20Object%20Reference))
  (return (.Location (Math|Transform|BreakTransform (Transformation|GetRelativeTransform Target)))))
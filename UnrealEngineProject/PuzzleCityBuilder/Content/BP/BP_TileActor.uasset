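; BP_TileActor is a clickable map tile that shows one building type: Road, House, Store, Hospital or School.
; Clicking the tile or any of its building components copies the current tile type from the first BP_BuildManager, found on BeginPlay, and prints it.
; Tick polls for a state change, then hides all five building components and reveals the matching one.
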(event OnClicked(Tile)
  (params (TouchedComponent :type Primitive%20Component%20Object%20Reference) (ButtonPressed :type Key%20Structure :default "None"))
  (Variables|Default|SetCurrentTileState (Variables|/Game/BP/BP_BuildManager.BP_BuildManager_C|GetCurrentTileType (Utilities|Array|Get(acopy) (stale EventBeginPlay _outactors))))
  (Development|PrintString (Utilities|String|EnumtoString (Variables|Default|GetCurrentTileState))))

(event OnClicked(Hospital)
  (params (TouchedComponent :type Primitive%20Component%20Object%20Reference) (ButtonPressed :type Key%20Structure :default "None"))
  (Variables|Default|SetCurrentTileState (Variables|/Game/BP/BP_BuildManager.BP_BuildManager_C|GetCurrentTileType (Utilities|Array|Get(acopy) (stale EventBeginPlay _outactors))))
  (Development|PrintString (Utilities|String|EnumtoString (Variables|Default|GetCurrentTileState))))

(event OnClicked(School)
  (params (TouchedComponent :type Primitive%20Component%20Object%20Reference) (ButtonPressed :type Key%20Structure :default "None"))
  (Variables|Default|SetCurrentTileState (Variables|/Game/BP/BP_BuildManager.BP_BuildManager_C|GetCurrentTileType (Utilities|Array|Get(acopy) (stale EventBeginPlay _outactors))))
  (Development|PrintString (Utilities|String|EnumtoString (Variables|Default|GetCurrentTileState))))

(event OnClicked(Store)
  (params (TouchedComponent :type Primitive%20Component%20Object%20Reference) (ButtonPressed :type Key%20Structure :default "None"))
  (Variables|Default|SetCurrentTileState (Variables|/Game/BP/BP_BuildManager.BP_BuildManager_C|GetCurrentTileType (Utilities|Array|Get(acopy) (stale EventBeginPlay _outactors))))
  (Development|PrintString (Utilities|String|EnumtoString (Variables|Default|GetCurrentTileState))))

(event OnClicked(House)
  (params (TouchedComponent :type Primitive%20Component%20Object%20Reference) (ButtonPressed :type Key%20Structure :default "None"))
  (Variables|Default|SetCurrentTileState (Variables|/Game/BP/BP_BuildManager.BP_BuildManager_C|GetCurrentTileType (Utilities|Array|Get(acopy) (stale EventBeginPlay _outactors))))
  (Development|PrintString (Utilities|String|EnumtoString (Variables|Default|GetCurrentTileState))))

(event OnClicked(Road)
  (params (TouchedComponent :type Primitive%20Component%20Object%20Reference) (ButtonPressed :type Key%20Structure :default "None"))
  (Variables|Default|SetCurrentTileState (Variables|/Game/BP/BP_BuildManager.BP_BuildManager_C|GetCurrentTileType (Utilities|Array|Get(acopy) (stale EventBeginPlay _outactors))))
  (Development|PrintString (Utilities|String|EnumtoString (Variables|Default|GetCurrentTileState))))

(event Custom|OnTileChange
  (CallFunction|TurnOffAllTiles)
  (switch Utilities|FlowControl|Switch|SwitchonTileState (Variables|Default|GetCurrentTileState)
    (:NewEnumerator1
      (Rendering|SetVisibility (Variables|Default|GetRoad) true false))
    (:NewEnumerator2
      (Rendering|SetVisibility (Variables|Default|GetHouse) true false))
    (:NewEnumerator3
      (Rendering|SetVisibility (Variables|Default|GetStore) true false))
    (:NewEnumerator4
      (Rendering|SetVisibility (Variables|Default|GetHospital) true false))
    (:NewEnumerator5
      (Rendering|SetVisibility (Variables|Default|GetSchool) true false))))

(event Custom|TurnOffAllTiles
  (Rendering|SetVisibility (Variables|Default|GetStore) false false)
  (Rendering|SetVisibility (Variables|Default|GetSchool) false false)
  (Rendering|SetVisibility (Variables|Default|GetRoad) false false)
  (Rendering|SetVisibility (Variables|Default|GetHouse) false false)
  (Rendering|SetVisibility (Variables|Default|GetHospital) false false))

(event EventBeginPlay
  (bind _outactors (Actor|GetAllActorsOfClass "/Game/BP/BP_BuildManager.BP_BuildManager_C")))

(event EventTick
  (params (DeltaSeconds :type Float%20%28single-precision%29))
  (if (!= (Variables|Default|GetLastTileState) (Math|Conversions|ToInteger(Byte) (Variables|Default|GetCurrentTileState)))
    (Variables|Default|SetLastTileState (Variables|Default|GetCurrentTileState))
    (CallFunction|OnTileChange)))

(fn ConstructionScript)
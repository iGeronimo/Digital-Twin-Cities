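; BP_TurnManager counts down the turns left and disables building when they run out.
; On BeginPlay it caches the first top-level BP_UIBuildButtons widget and has it set its turn text.
; OnTurnCompleted decrements TurnsLeft and refreshes that text, then sets CanBuild to false on the BP_BuildManager actor once the count is no longer above zero.
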(event Custom|OnTurnCompleted
  (bind _result (Math|Integer|DecrementInt (Variables|Default|GetTurnsLeft))
    (:%20%20
      (if (> _result 0)
        (Default|SetTurnText (Variables|Default|GetUIComponent))
        (else
          (Default|SetTurnText (Variables|Default|GetUIComponent))
          (bind _returnvalue (Actor|GetActorOfClass "/Game/BP/BP_BuildManager.BP_BuildManager_C"))
          (Variables|/Game/BP/BP_BuildManager.BP_BuildManager_C|SetCanBuild _returnvalue false))))))

(event EventBeginPlay
  (bind _foundwidgets (Widget|GetAllWidgetsOfClass "/Game/BP/BP_UIBuildButtons.BP_UIBuildButtons_C" true))
  (bind _output_get (Variables|Default|SetUIComponent (Utilities|Array|Get(acopy) _foundwidgets)))
  (Default|SetTurnText _output_get))

(fn ConstructionScript)
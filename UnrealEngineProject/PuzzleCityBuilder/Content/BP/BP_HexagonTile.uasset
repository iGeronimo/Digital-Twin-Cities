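; Hexagon city-building tile that shows one of five building types: road, house, store, hospital or school.
; Clicking copies the selected type from BP_BuildManager; Tick spots the change, enables only that building's mesh and query collision, then asks BP_NecessityManager to check amenity zones.
; CheckNeighbours adds unchecked overlapping tiles of a requested type to the manager's NewObjects, while AddPointAndCheck increments points and marks the tile checked.
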(event OnClicked(Tile)
  (params (TouchedComponent :type Primitive%20Component%20Object%20Reference) (ButtonPressed :type Key%20Structure :default "None"))
  ;[1 1 1] OnClick behaviour
  (Variables|Default|SetCurrentTileState (Variables|/Game/BP/BP_BuildManager.BP_BuildManager_C|GetCurrentTileType (Utilities|Array|Get(acopy) (stale EventBeginPlay _outactors))))
  (Development|PrintString (Utilities|String|EnumtoString (Variables|Default|GetCurrentTileState))))

(event OnClicked(Hospital)
  (params (TouchedComponent :type Primitive%20Component%20Object%20Reference) (ButtonPressed :type Key%20Structure :default "None"))
  ;[1 1 1] OnClick behaviour
  (Variables|Default|SetCurrentTileState (Variables|/Game/BP/BP_BuildManager.BP_BuildManager_C|GetCurrentTileType (Utilities|Array|Get(acopy) (stale EventBeginPlay _outactors))))
  (Development|PrintString (Utilities|String|EnumtoString (Variables|Default|GetCurrentTileState))))

(event OnClicked(School)
  (params (TouchedComponent :type Primitive%20Component%20Object%20Reference) (ButtonPressed :type Key%20Structure :default "None"))
  ;[1 1 1] OnClick behaviour
  (Variables|Default|SetCurrentTileState (Variables|/Game/BP/BP_BuildManager.BP_BuildManager_C|GetCurrentTileType (Utilities|Array|Get(acopy) (stale EventBeginPlay _outactors))))
  (Development|PrintString (Utilities|String|EnumtoString (Variables|Default|GetCurrentTileState))))

(event OnClicked(Store)
  (params (TouchedComponent :type Primitive%20Component%20Object%20Reference) (ButtonPressed :type Key%20Structure :default "None"))
  ;[1 1 1] OnClick behaviour
  (Variables|Default|SetCurrentTileState (Variables|/Game/BP/BP_BuildManager.BP_BuildManager_C|GetCurrentTileType (Utilities|Array|Get(acopy) (stale EventBeginPlay _outactors))))
  (Development|PrintString (Utilities|String|EnumtoString (Variables|Default|GetCurrentTileState))))

(event OnClicked(House)
  (params (TouchedComponent :type Primitive%20Component%20Object%20Reference) (ButtonPressed :type Key%20Structure :default "None"))
  ;[1 1 1] OnClick behaviour
  (Variables|Default|SetCurrentTileState (Variables|/Game/BP/BP_BuildManager.BP_BuildManager_C|GetCurrentTileType (Utilities|Array|Get(acopy) (stale EventBeginPlay _outactors))))
  (Development|PrintString (Utilities|String|EnumtoString (Variables|Default|GetCurrentTileState))))

(event OnClicked(Road)
  (params (TouchedComponent :type Primitive%20Component%20Object%20Reference) (ButtonPressed :type Key%20Structure :default "None"))
  ;[1 1 1] OnClick behaviour
  (Variables|Default|SetCurrentTileState (Variables|/Game/BP/BP_BuildManager.BP_BuildManager_C|GetCurrentTileType (Utilities|Array|Get(acopy) (stale EventBeginPlay _outactors))))
  (Development|PrintString (Utilities|String|EnumtoString (Variables|Default|GetCurrentTileState))))

(event Custom|CheckNeighbours
  (params (WhatTileToCheck :type TileState%20Enum :default "NewEnumerator0"))
  ;[1 0.9594 0.3846] CheckNeighbours
  (for _array_element (Collision|GetOverlappingActors (Variables|Default|GetNeighbourCheckHitbox) "BP_HexagonTile_C" :!class /Script/Engine.PrimitiveComponent)
    (bind _asbp_hexagon_tile (Utilities|Casting|CastToBP_HexagonTile _array_element))
    (if (not (Variables|BP_HexagonTile_C|GetIsChecked _asbp_hexagon_tile))
      (if (== (Math|Conversions|ToInteger(Byte) WhatTileToCheck) (Math|Conversions|ToInteger(Byte) (Variables|BP_HexagonTile_C|GetCurrentTileState _asbp_hexagon_tile)))
        (bind _returnvalue (Actor|GetActorOfClass "/Game/BP/BP_NecessityManager.BP_NecessityManager_C"))
        (Utilities|Array|Add (Variables|/Game/BP/BP_NecessityManager.BP_NecessityManager_C|GetNewObjects _returnvalue) _asbp_hexagon_tile)))))

(event Custom|AddPointAndCheck
  ;[1 0.2818 0] AddPointsAndCheck
  (Math|Integer|IncrementInt (Variables|Default|GetTilePoints)
    (:%20%20
      (Variables|Default|SetIsChecked true))))

(event Custom|TurnOffAllTiles
  (bind _hospital (Variables|Default|GetHospital))
  ;[0 0.1293 1] TurnOffAllBuildings
  (Rendering|SetVisibility (Variables|Default|GetStore) false false)
  (Rendering|SetVisibility (Variables|Default|GetSchool) false false)
  (Rendering|SetVisibility (Variables|Default|GetRoad) false false)
  (Rendering|SetVisibility (Variables|Default|GetHouse) false false)
  (Rendering|SetVisibility _hospital false false)
  (Collision|SetCollisionEnabled _hospital "NoCollision"))

(event Custom|OnTileChange
  (bind _road (Variables|Default|GetRoad))
  (bind _house (Variables|Default|GetHouse))
  (bind _store (Variables|Default|GetStore))
  (bind _hospital (Variables|Default|GetHospital))
  (bind _school (Variables|Default|GetSchool))
  ;[0 1 0.01166] BuildingEnabler
  (CallFunction|TurnOffAllTiles)
  (switch Utilities|FlowControl|Switch|SwitchonTileState (Variables|Default|GetCurrentTileState)
    (:NewEnumerator1
      (Rendering|SetVisibility _road true false)
      (Collision|SetCollisionEnabled _road "QueryOnly"))
    (:NewEnumerator2
      (Rendering|SetVisibility _house true false)
      (Collision|SetCollisionEnabled _house "QueryOnly"))
    (:NewEnumerator3
      (Rendering|SetVisibility _store true false)
      (Collision|SetCollisionEnabled _store "QueryOnly"))
    (:NewEnumerator4
      (Rendering|SetVisibility _hospital true false)
      (Collision|SetCollisionEnabled _hospital "QueryOnly"))
    (:NewEnumerator5
      (Rendering|SetVisibility _school true false)
      (Collision|SetCollisionEnabled _school "QueryOnly")))
  (bind _returnvalue (Actor|GetActorOfClass "/Game/BP/BP_NecessityManager.BP_NecessityManager_C"))
  (Default|CheckAmenityZones _returnvalue self))

(event EventBeginPlay
  ;[1 0.02604 0] Initialize
  (CallFunction|OnTileChange)
  (for _array_element (Utilities|Array|MakeArray (Variables|Default|GetSchool) (Variables|Default|GetStore) (Variables|Default|GetHouse) (Variables|Default|GetRoad) (Variables|Default|GetHospital))
    (Transformation|SetRelativeRotation _array_element "0.000000,60.000000,0.000000" false false))
  (bind _outactors (Actor|GetAllActorsOfClass "/Game/BP/BP_BuildManager.BP_BuildManager_C")))

(event EventTick
  (params (DeltaSeconds :type Float%20%28single-precision%29))
  ;[1 0.7633 0] TileChangeStateCheck
  (if (!= (Variables|Default|GetLastTileState) (Math|Conversions|ToInteger(Byte) (Variables|Default|GetCurrentTileState)))
    (Variables|Default|SetLastTileState (Variables|Default|GetCurrentTileState))
    (CallFunction|OnTileChange)))

(fn ConstructionScript)
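; BP_TestFuncManager is a debug helper that binds keys to cheats for the turn and building systems.
; Releasing O gives BP_TurnManager a very large turn count, while P resets it to a small one.
; Both keys also re-enable building on BP_BuildManager and refresh the turn text on the BP_UIBuildButtons widget, finding each target by class lookup.
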(event Input|KeyboardEvents|P
  (params (Key :type Key%20Structure :default "None"))
  (:Released
    (bind _returnvalue (Actor|GetActorOfClass "/Game/BP/BP_TurnManager.BP_TurnManager_C"))
    (Variables|/Game/BP/BP_TurnManager.BP_TurnManager_C|SetTurnsLeft _returnvalue 5)
    (bind _returnvalue_2 (Actor|GetActorOfClass "/Game/BP/BP_BuildManager.BP_BuildManager_C"))
    (Variables|/Game/BP/BP_BuildManager.BP_BuildManager_C|SetCanBuild _returnvalue_2 true)
    (bind _foundwidgets (Widget|GetAllWidgetsOfClass "/Game/BP/BP_UIBuildButtons.BP_UIBuildButtons_C" true))
    (Default|SetTurnText (Utilities|Array|Get(acopy) _foundwidgets))))

(event Input|KeyboardEvents|O
  (params (Key :type Key%20Structure :default "None"))
  (:Released
    (bind _returnvalue (Actor|GetActorOfClass "/Game/BP/BP_TurnManager.BP_TurnManager_C"))
    (Variables|/Game/BP/BP_TurnManager.BP_TurnManager_C|SetTurnsLeft _returnvalue 1000)
    (bind _returnvalue_2 (Actor|GetActorOfClass "/Game/BP/BP_BuildManager.BP_BuildManager_C"))
    (Variables|/Game/BP/BP_BuildManager.BP_BuildManager_C|SetCanBuild _returnvalue_2 true)
    (bind _foundwidgets (Widget|GetAllWidgetsOfClass "/Game/BP/BP_UIBuildButtons.BP_UIBuildButtons_C" true))
    (Default|SetTurnText (Utilities|Array|Get(acopy) _foundwidgets))))

(fn ConstructionScript)
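; House generator Blueprint that stacks instanced static mesh modules into a randomized house, built in the construction script and rebuilt on pressing H.
; GenerateHouse clears the ground, floor and roof instances, then measures module heights from mesh bounding boxes.
; It places a random ground mesh, repeated floors and a random roof at an accumulating height, with floor count bounded by MaxFloors.
; The ground height uses its own random pick, independent of the chosen mesh.
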(event EventBeginPlay)

(event Collision|EventActorBeginOverlap
  (params (OtherActor :type Actor%20Object%20Reference)))

(event EventTick
  (params (DeltaSeconds :type Float%20%28single-precision%29)))

(event Input|KeyboardEvents|H
  (params (Key :type Key%20Structure :default "None"))
  (:Pressed
    (CallFunction|GenerateHouse)))

(fn ConstructionScript
  (CallFunction|GenerateHouse))

(fn GenerateHouse
  (bind _returnvalue (Math|Random|RandomIntegerinRange 0 1))
  (Components|InstancedStaticMesh|ClearInstances (Variables|Default|GetGroundModule))
  (Components|InstancedStaticMesh|ClearInstances (Variables|Default|GetFloorModule))
  (Components|InstancedStaticMesh|ClearInstances (Variables|Default|GetRoofModule))
  (bind _output_get (Variables|Default|SetModules (Utilities|Array|MakeArray (Variables|Default|GetGroundModule_01) (Variables|Default|GetGroundModule_02) (Variables|Default|GetFloorModule_01) (Variables|Default|GetRoofModule_01) (Variables|Default|GetRoofModule_02) (Variables|Default|GetRoofModule_03))))
  (for _array_element _output_get
    (Utilities|Array|Add (Variables|Default|GetModuleHeights) (- (.z (.Max (Utilities|Struct|BreakBox (StaticMesh|GetBoundingBox _array_element)))) (.z (.Min (Utilities|Struct|BreakBox (StaticMesh|GetBoundingBox _array_element)))))))
  (bind _output_get_2 (Variables|Default|SetNumFloors (Math|Random|RandomIntegerinRange 2 (- (Math|Integer|Max(Integer) (Variables|Default|GetMaxFloors) 3) 1))))
  (for _index (range 0 _output_get_2)
    (switch int _index
      (:Default
        (if (== _index (Variables|Default|GetNumFloors))
          (Components|StaticMesh|SetStaticMesh (Variables|Default|GetRoofModule) (Utilities|Array|Get(acopy) (Variables|Default|GetModules) (Math|Random|RandomIntegerinRange 3 5)))
          (Components|InstancedStaticMesh|AddInstance (Variables|Default|GetRoofModule) (Math|Transform|MakeTransform (Math|Vector|MakeVector 0.0 0.0 (Variables|Default|GetCurrentHeight)) "0.000000,90.000000,0.000000") false)
          (else
            (Components|InstancedStaticMesh|AddInstance (Variables|Default|GetFloorModule) (Math|Transform|MakeTransform (Math|Vector|MakeVector 0.0 0.0 (Variables|Default|GetCurrentHeight)) "0.000000,90.000000,0.000000") false)
            (Variables|Default|SetCurrentHeight (+ (Variables|Default|GetCurrentHeight) (Utilities|Array|Get(acopy) (Variables|Default|GetModuleHeights) 2))))))
      (:0
        (Components|StaticMesh|SetStaticMesh (Variables|Default|GetGroundModule) (Utilities|Array|Get(acopy) (Variables|Default|GetModules) _returnvalue))
        (Components|InstancedStaticMesh|AddInstance (Variables|Default|GetGroundModule) (Math|Transform|MakeTransform "0, 0, 0" "0.000000,90.000000,0.000000") false)
        (Variables|Default|SetCurrentHeight (+ (Variables|Default|GetCurrentHeight) (Utilities|Array|Get(acopy) (Variables|Default|GetModuleHeights) _returnvalue))))))
  (Variables|Default|SetCurrentHeight 0.0))
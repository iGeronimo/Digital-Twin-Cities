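; BP_SmogControl is an actor that fades a smog effect in and out according to its EnableSmog flag.
; On BeginPlay it finds the level's height fog and post process volume, then creates dynamic materials for a post process blendable and its SmogVolume.
; Tick steps SmogOpacity by a fixed per-frame amount, driving post process opacity, volume fog thickness and volumetric fog distance together.
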(event EventBeginPlay
  (bind _returnvalue (Actor|GetActorOfClass "/Script/Engine.ExponentialHeightFog"))
  (Variables|Default|SetExpFog _returnvalue)
  (bind _returnvalue_2 (Rendering|Material|CreateDynamicMaterialInstance "/Game/Shaders/Smog/PPI_Smog_v02.PPI_Smog_v02" "None" "None" :!class /Script/Engine.KismetMaterialLibrary))
  (Variables|Default|SetPP_Material _returnvalue_2)
  (bind _returnvalue_3 (Actor|GetActorOfClass "/Script/Engine.PostProcessVolume"))
  (Utilities|Struct|SetmembersinPostProcessSettings (Variables|/Script/Engine.PostProcessVolume|GetSettings _returnvalue_3) (Utilities|Struct|MakeWeightedBlendables (Utilities|Array|MakeArray (Utilities|Struct|MakeWeightedBlendable 1.0 (Variables|Default|GetPP_Material)))))
  (bind _returnvalue_4 (Rendering|Material|CreateDynamicMaterialInstance (Variables|Default|GetSmogVolume) 0 "/Game/Shaders/Smog/VI_Smog.VI_Smog" "None" :!class /Script/Engine.PrimitiveComponent))
  (Variables|Default|SetVolume_Material _returnvalue_4))

(event Collision|EventActorBeginOverlap
  (params (OtherActor :type Actor%20Object%20Reference)))

(event EventTick
  (params (DeltaSeconds :type Float%20%28single-precision%29))
  (if (Variables|Default|GetEnableSmog)
    (if (< (Variables|Default|GetSmogOpacity) 1.0)
      (Variables|Default|SetSmogOpacity (+ (Variables|Default|GetSmogOpacity) 0.01))
      (Rendering|Material|SetScalarParameterValue (Variables|Default|GetPP_Material) "Opacity" (Math|Float|MapRangeClamped (Variables|Default|GetSmogOpacity) 0.0 1.0 0.0 0.4) :!class /Script/Engine.MaterialInstanceDynamic :!label _label)
      (Rendering|Material|SetScalarParameterValue (Variables|Default|GetVolume_Material) "Fog Thikness" (Variables|Default|GetSmogOpacity) :!class /Script/Engine.MaterialInstanceDynamic)
      (Class|ExponentialHeightFogComponent|SetVolumetricFogDistance (Variables|/Script/Engine.ExponentialHeightFog|GetComponent (Variables|Default|GetExpFog)) (Math|Float|MapRangeClamped (Variables|Default|GetSmogOpacity) 0.0 1.0 0.0 2e+04)))
    (elif (> (Variables|Default|GetSmogOpacity) 0.0)
      (Variables|Default|SetSmogOpacity (- (Variables|Default|GetSmogOpacity) 0.01))
      (goto _label))))

(fn ConstructionScript)
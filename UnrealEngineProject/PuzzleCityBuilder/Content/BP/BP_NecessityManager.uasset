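; BP_NecessityManager recalculates amenity coverage and scoring for a hex-tile town builder through its CheckAmenityZones event.
; It resets tile points, gathers Store, Hospital and School tiles, then flood-fills from each through road neighbours up to AmenityRange, awarding points to reached tiles.
; It then recomputes house points and score, refreshing the score text, happiness meter and tile range shaders.
; Each pass repeatedly scans all BP_HexagonTile actors rather than updating incrementally.
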(event Custom|CheckAmenityZones
  (params (ChangedBuilding :type BP%20Hexagon%20Tile%20Object%20Reference))
  ;[1 1 1] CheckNecessityRange
  (bind _outactors (Actor|GetAllActorsOfClass "/Game/BP/BP_HexagonTile.BP_HexagonTile_C"))
  (for _array_element _outactors
    (Variables|/Game/BP/BP_HexagonTile.BP_HexagonTile_C|SetTilePoints _array_element 0))
  (Utilities|Array|Clear (Variables|Default|GetCurrentObjects))
  (Utilities|Array|Clear (Variables|Default|GetNecessityTiles))
  (bind _outactors_2 (Actor|GetAllActorsOfClass "/Game/BP/BP_HexagonTile.BP_HexagonTile_C"))
  (for _array_element_2 _outactors_2
    (switch Utilities|FlowControl|Switch|SwitchonTileState (Variables|/Game/BP/BP_HexagonTile.BP_HexagonTile_C|GetCurrentTileState _array_element_2)
      (:NewEnumerator3
        _)
      (:NewEnumerator4
        _)
      (:NewEnumerator5
        _))
    (Utilities|Array|AddUnique (Variables|Default|GetNecessityTiles) _array_element_2))
  (for _array_element_3 (Variables|Default|GetNecessityTiles)
    (Utilities|Array|AddUnique (Variables|Default|GetCurrentObjects) _array_element_3)
    (for _index (range 0 (Variables|Default|GetAmenityRange))
      (for _array_element_4 (Variables|Default|GetCurrentObjects)
        (Default|CheckNeighbours _array_element_4 "NewEnumerator1"))
      (for _array_element_5 (Variables|Default|GetNewObjects)
        (Default|AddPointsandCheck _array_element_5 (Variables|/Game/BP/BP_HexagonTile.BP_HexagonTile_C|GetCurrentTileState _array_element_3)))
      (Utilities|Array|Clear (Variables|Default|GetCurrentObjects))
      (Variables|Default|SetCurrentObjects (Variables|Default|GetNewObjects))
      (Utilities|Array|Clear (Variables|Default|GetNewObjects)))
    (bind _outactors_3 (Actor|GetAllActorsOfClass "/Game/BP/BP_HexagonTile.BP_HexagonTile_C"))
    (for _array_element_6 _outactors_3
      (Variables|/Game/BP/BP_HexagonTile.BP_HexagonTile_C|SetIsChecked _array_element_6 false)
      (Utilities|Array|Clear (Variables|Default|GetCurrentObjects))))
  (bind _outactors_4 (Actor|GetAllActorsOfClass "/Game/BP/BP_HexagonTile.BP_HexagonTile_C"))
  (for _array_element_7 _outactors_4
    (Variables|/Game/BP/BP_HexagonTile.BP_HexagonTile_C|SetHospitalPoint _array_element_7 false)
    (Variables|/Game/BP/BP_HexagonTile.BP_HexagonTile_C|SetSchoolPoint _array_element_7 false)
    (Variables|/Game/BP/BP_HexagonTile.BP_HexagonTile_C|SetStorePoint _array_element_7 false)
    (if (== (Math|Conversions|ToInteger(Byte) (Utilities|Enum|LiteralenumTileState "NewEnumerator2")) (Variables|/Game/BP/BP_HexagonTile.BP_HexagonTile_C|GetCurrentTileState _array_element_7))
      (Default|HousePoints _array_element_7)))
  (Variables|Default|SetScore 0)
  (for _array_element_8 _outactors_4
    (Default|SetHousePoints _array_element_8))
  (bind _foundwidgets (Widget|GetAllWidgetsOfClass "/Game/BP/BP_UIBuildButtons.BP_UIBuildButtons_C" true))
  (for _array_element_9 _foundwidgets
    (Default|SetScoreText _array_element_9)
    (Default|SetHappinessMeter _array_element_9))
  (bind _outactors_5 (Actor|GetAllActorsOfClass "/Game/BP/BP_HexagonTile.BP_HexagonTile_C"))
  (for _array_element_10 _outactors_5
    (Default|SetRangeShader _array_element_10)))

(fn ConstructionScript)
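; BP_RoadManager rebuilds spline roads across BP_HexagonTile actors when F is pressed, destroying its old spline and spline mesh components first.
; CheckRoads walks overlapping road-state tiles in both directions, prepending or appending them into ordered chains, and CheckNeighbours stops expanding at tiles with three or more road neighbours.
; CreateSpline places raised points at chain ends and between tile centres, then AddSplineMeshes sets tangents and adds a spline mesh per segment.
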(event EventBeginPlay)

(event Collision|EventActorBeginOverlap
  (params (OtherActor :type Actor%20Object%20Reference)))

(event EventTick
  (params (DeltaSeconds :type Float%20%28single-precision%29)))

(event Input|KeyboardEvents|F
  (params (Key :type Key%20Structure :default "None"))
  (:Pressed
    (Utilities|Array|Clear (Variables|Default|GetRoadsChecked))
    (Variables|Default|SetRoadSplines (Actor|GetComponentsByClass "/Script/Engine.SplineComponent"))
    (Variables|Default|SetRoadSplineMeshes (Actor|GetComponentsByClass "/Script/Engine.SplineMeshComponent"))
    (for _array_element (Variables|Default|GetRoadSplines)
      (Components|DestroyComponent _array_element))
    (for _array_element_2 (Variables|Default|GetRoadSplineMeshes)
      (Components|DestroyComponent _array_element_2))
    (CallFunction|CheckRoads)))

(fn ConstructionScript)

(fn CheckRoads
  (Utilities|Array|Clear (Variables|Default|GetIntersections))
  (bind _outactors (Actor|GetAllActorsOfClass "/Game/BP/BP_HexagonTile.BP_HexagonTile_C"))
  (for _array_element _outactors
    (if (Utilities|Enum|Equal(Enum) (Variables|/Game/BP/BP_HexagonTile.BP_HexagonTile_C|GetCurrentTileState _array_element) "NewEnumerator1")
      (CallFunction|CheckNeighbours _array_element)
      (bind _output_get (Variables|Default|SetRoadsToCheck (Variables|Default|GetRoadsToCheckTemp)))
      (Variables|Default|SetRoadsToCheckDirection (Variables|Default|GetRoadsToCheckDirectionTemp))
      (if (Utilities|Array|IsNotEmpty _output_get)
        (Utilities|Array|AddUnique (Variables|Default|GetRoads) _array_element)
        (Utilities|Array|AddUnique (Variables|Default|GetRoadsChecked) _array_element)
        (CallFunction|ClearTempArrays)
        (while (Utilities|Array|IsNotEmpty (Variables|Default|GetRoadsToCheck))
          (for (_array_element_2 _array_index) (Variables|Default|GetRoadsToCheck)
            (CallFunction|CheckNeighbours _array_element_2 (Utilities|Array|Get(acopy) (Variables|Default|GetRoadsToCheckDirection) _array_index)))
          (Variables|Default|SetRoadsToCheck (Variables|Default|GetRoadsToCheckTemp))
          (Variables|Default|SetRoadsToCheckDirection (Variables|Default|GetRoadsToCheckDirectionTemp))
          (CallFunction|ClearTempArrays))
        (CallFunction|CreateSpline)
        (Utilities|Array|Clear (Variables|Default|GetRoads))))))

(fn CheckNeighbours
  (params (InputTile :type BP%20Hexagon%20Tile%20Object%20Reference) (InputDirection :type Integer))
  (bind _overlappingactors (Collision|GetOverlappingActors InputTile "/Game/BP/BP_HexagonTile.BP_HexagonTile_C" :!class /Script/Engine.Actor))
  (bind _roadstocheckdirectiontemp (Variables|Default|GetRoadsToCheckDirectionTemp))
  (bind _array_element (Utilities|Array|ForEachLoopwithBreak _overlappingactors :!label _label)
    (:LoopBody
      (bind _asbp_hexagon_tile (Utilities|Casting|CastToBP_HexagonTile _array_element))
      (if (< (LocalVariables|GetRoadCount) 3)
        (if (Utilities|Enum|Equal(Enum) (Variables|/Game/BP/BP_HexagonTile.BP_HexagonTile_C|GetCurrentTileState _asbp_hexagon_tile) "NewEnumerator1")
          (Math|Integer|IncrementInt (LocalVariables|GetRoadCount)))
        (else
          (goto _label Break))))
    (:Completed
      (if (< (LocalVariables|GetRoadCount) 3)
        (for _array_element_2 _overlappingactors
          (bind _asbp_hexagon_tile_2 (Utilities|Casting|CastToBP_HexagonTile _array_element_2))
          (if (Utilities|Enum|Equal(Enum) (Variables|/Game/BP/BP_HexagonTile.BP_HexagonTile_C|GetCurrentTileState _asbp_hexagon_tile_2) "NewEnumerator1")
            (if (not (Utilities|Array|ContainsItem (Variables|Default|GetRoadsChecked) _asbp_hexagon_tile_2))
              (bind _returnvalue (Utilities|Array|Add (Variables|Default|GetRoadsToCheckTemp) _asbp_hexagon_tile_2))
              (if (!= InputDirection 0)
                (Utilities|Array|Add _roadstocheckdirectiontemp InputDirection)
                (else
                  (Utilities|Array|Add _roadstocheckdirectiontemp (+ _returnvalue 1)))))))
        (CallFunction|AddRoadtoArray InputTile)))))

(fn ClearTempArrays
  (Utilities|Array|Clear (Variables|Default|GetRoadsToCheckTemp))
  (Utilities|Array|Clear (Variables|Default|GetRoadsToCheckDirectionTemp)))

(fn AddRoadtoArray
  (params (InputRoad :type BP%20Hexagon%20Tile%20Object%20Reference))
  (bind _roads (Variables|Default|GetRoads))
  (bind _roadstocheck (Variables|Default|GetRoadsToCheck))
  (bind _returnvalue (Utilities|Array|FindItem _roadstocheck InputRoad))
  (Utilities|Array|Add (Variables|Default|GetRoadsChecked) InputRoad)
  (if (>= _returnvalue 0)
    (switch int (Utilities|Array|Get(acopy) (Variables|Default|GetRoadsToCheckDirection) _returnvalue)
      (:1
        (Utilities|Array|Insert _roads InputRoad))
      (:2
        (Utilities|Array|Insert _roads InputRoad (+ (Utilities|Array|LastIndex _roads) 1))))))

(fn CreateSpline
  (bind _splinepointlocations (Variables|Default|GetSplinePointLocations))
  (bind _roads (Variables|Default|GetRoads))
  (bind _returnvalue (AddComponent|AddSplineComponent false))
  (bind _output_get (LocalVariables|SetSpline _returnvalue))
  (Spline|ClearSplinePoints _output_get true)
  (for (_array_element _array_index) (Variables|Default|GetRoads)
    (Utilities|Array|Add (Variables|Default|GetRoadLocations) (Transformation|GetWorldLocation (Variables|/Game/BP/BP_HexagonTile.BP_HexagonTile_C|GetDefaultSceneRoot _array_element)))
    (if (Utilities|Array|IsValidIndex _roads (- _array_index 1))
      (Utilities|Array|Add _splinepointlocations (/ (+ (Transformation|GetWorldLocation (Variables|/Script/Engine.Actor|GetRootComponent _array_element)) (Transformation|GetWorldLocation (Variables|/Script/Engine.Actor|GetRootComponent (Utilities|Array|Get(acopy) (Variables|Default|GetRoads) (- _array_index 1)))) "0.000000,0.000000,110.000000") "2.000000,2.000000,1.000000"))
      (Spline|AddSplinePoint (LocalVariables|GetSpline) (/ (+ (Transformation|GetWorldLocation (Variables|/Script/Engine.Actor|GetRootComponent _array_element)) (Transformation|GetWorldLocation (Variables|/Script/Engine.Actor|GetRootComponent (Utilities|Array|Get(acopy) (Variables|Default|GetRoads) (- _array_index 1)))) "0.000000,0.000000,110.000000") "2.000000,2.000000,1.000000") "World" true)
      (if (not (Utilities|Array|IsValidIndex _roads (+ _array_index 1)))
        (Utilities|Array|Add (Variables|Default|GetSplinePointLocations) (+ (Transformation|GetWorldLocation (Variables|/Script/Engine.Actor|GetRootComponent _array_element)) "0.000000,0.000000,110.000000"))
        (Spline|AddSplinePoint (LocalVariables|GetSpline) (+ (Transformation|GetWorldLocation (Variables|/Script/Engine.Actor|GetRootComponent _array_element)) "0.000000,0.000000,110.000000") "World" true))
      (else
        (Utilities|Array|Add _splinepointlocations (+ (Transformation|GetWorldLocation (Variables|/Script/Engine.Actor|GetRootComponent _array_element)) "0.000000,0.000000,110.000000"))
        (Spline|AddSplinePoint (LocalVariables|GetSpline) (+ (Transformation|GetWorldLocation (Variables|/Script/Engine.Actor|GetRootComponent _array_element)) "0.000000,0.000000,110.000000") "World" true))))
  (CallFunction|AddSplineMeshes (LocalVariables|GetSpline))
  (Utilities|Array|Clear (Variables|Default|GetRoadLocations))
  (Utilities|Array|Clear (Variables|Default|GetSplinePointLocations)))

(fn AddSplineMeshes
  (params (InputSpline :type Spline%20Component%20Object%20Reference))
  (bind _returnvalue (Spline|GetNumberOfSplinePoints InputSpline))
  (bind _splinepointlocations (Variables|Default|GetSplinePointLocations))
  (bind _splinepointlocations_2 (Variables|Default|GetSplinePointLocations))
  (bind _output (Utilities|Array|Get(acopy) _splinepointlocations))
  (bind _output_2 (Utilities|Array|Get(acopy) _splinepointlocations 1))
  (bind _returnvalue_2 (- _returnvalue 1))
  (bind _returnvalue_3 (- _output_2 _output))
  (bind _returnvalue_4 (* _returnvalue_3 "2.000000,2.000000,0.000000"))
  (LocalVariables|SetSpline InputSpline)
  (for _index (range 0 _returnvalue_2)
    (LocalVariables|SetCurrentIndex _index)
    (switch int (LocalVariables|GetCurrentIndex)
      (:Default
        (if (== (LocalVariables|GetCurrentIndex) _returnvalue_2)
          (Spline|SetTangentsatSplinePoint (LocalVariables|GetSpline) (LocalVariables|GetCurrentIndex) (* (- (Utilities|Array|Get(acopy) _splinepointlocations_2 (LocalVariables|GetCurrentIndex)) (Utilities|Array|Get(acopy) _splinepointlocations_2 (- (LocalVariables|GetCurrentIndex) 1))) "2.000000,2.000000,0.000000") (* (- (Utilities|Array|Get(acopy) _splinepointlocations_2 (LocalVariables|GetCurrentIndex)) (Utilities|Array|Get(acopy) _splinepointlocations_2 (- (LocalVariables|GetCurrentIndex) 1))) "2.000000,2.000000,0.000000") "World" true)
          (else
            (Spline|SetTangentsatSplinePoint (LocalVariables|GetSpline) (LocalVariables|GetCurrentIndex) (* (Utilities|Operators|Subtract (Utilities|Array|Get(acopy) (Variables|Default|GetRoadLocations) (LocalVariables|GetCurrentIndex)) (Utilities|Array|Get(acopy) (Variables|Default|GetSplinePointLocations) (LocalVariables|GetCurrentIndex)) "0.000000,0.000000,-110.000000") "2.000000,2.000000,0.000000") (* (Utilities|Operators|Subtract (Utilities|Array|Get(acopy) (Variables|Default|GetRoadLocations) (LocalVariables|GetCurrentIndex)) (Utilities|Array|Get(acopy) (Variables|Default|GetSplinePointLocations) (LocalVariables|GetCurrentIndex)) "0.000000,0.000000,-110.000000") "2.000000,2.000000,0.000000") "Local" true)))
        (bind _returnvalue_5 (AddComponent|AddSplineMeshComponent false))
        (SplineMesh|SetStartandEnd _returnvalue_5 (.Location (Spline|GetLocationandTangentatSplinePoint (LocalVariables|GetSpline) (- (LocalVariables|GetCurrentIndex) 1) "Local")) (.Tangent (Spline|GetLocationandTangentatSplinePoint (LocalVariables|GetSpline) (- (LocalVariables|GetCurrentIndex) 1) "Local")) (.Location (Spline|GetLocationandTangentatSplinePoint (LocalVariables|GetSpline) (LocalVariables|GetCurrentIndex) "Local")) (.Tangent (Spline|GetLocationandTangentatSplinePoint (LocalVariables|GetSpline) (LocalVariables|GetCurrentIndex) "Local")) true :!class /Script/Engine.SplineMeshComponent))
      (:0
        (Spline|SetTangentsatSplinePoint (LocalVariables|GetSpline) (LocalVariables|GetCurrentIndex) _returnvalue_4 _returnvalue_4 "Local" true)))))
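; Natural dressing actor that randomly scatters bush and tree instances over a rectangular area on BeginPlay, and again whenever K is pressed.
; GardenGeneration makes a few attempts per call, each adding a query-only capsule at a random position and yaw as an overlap probe.
; Overlapping probes are destroyed; clear ones remain, adding an instance to a randomly chosen one of four instanced static mesh components.
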(event EventBeginPlay
  (CallFunction|GardenGeneration "2000.000000,2000.000000,0.000000"))

(event Collision|EventActorBeginOverlap
  (params (OtherActor :type Actor%20Object%20Reference)))

(event EventTick
  (params (DeltaSeconds :type Float%20%28single-precision%29)))

(event Input|KeyboardEvents|K
  (params (Key :type Key%20Structure))
  (:Pressed
    (CallFunction|GardenGeneration "2000.000000,2000.000000,0.000000")))

(fn ConstructionScript)

(fn GardenGeneration
  (params (Area :type Vector))
  (bind (_x _y) (Math|Vector|BreakVector Area))
  (Variables|Default|SetISM_Array (Utilities|Array|MakeArray (Variables|Default|GetBush_01) (Variables|Default|GetBush_02) (Variables|Default|GetTree_01) (Variables|Default|GetTree_02)))
  (for _index (range 0 2)
    (bind _returnvalue (AddComponent|AddCapsuleComponent false (Math|Transform|MakeTransform (Math|Vector|MakeVector (* (Math|Random|RandomFloat) _x) (* (Math|Random|RandomFloat) _y) 0.0) (Math|Rotator|MakeRotator 0.0 0.0 (* (Math|Random|RandomFloat) 3.6e+02)) "1.000000,1.000000,1.000000")))
    (Collision|SetCollisionEnabled _returnvalue "QueryOnly")
    (bind _returnvalue_2 (Class|KismetSystemLibrary|ComponentOverlapComponents _returnvalue (Transformation|GetWorldTransform _returnvalue) (Utilities|Array|MakeArray "ObjectTypeQuery1") "/Script/Engine.CapsuleComponent"))
    (if _returnvalue_2
      (Components|DestroyComponent _returnvalue)
      (else
        (Components|InstancedStaticMesh|AddInstance (Utilities|Array|Get(acopy) (Variables|Default|GetISM_Array) (Math|Random|RandomInteger (Utilities|Array|Length (Variables|Default|GetISM_Array)))) (Transformation|GetRelativeTransform _returnvalue) false)))))
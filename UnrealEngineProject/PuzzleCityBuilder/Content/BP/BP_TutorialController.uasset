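; BP_TutorialController tracks progress through six tutorials, advancing a step counter as expected actions are completed.
; SetCurrentTutorialMap uses the current tutorial number to select the matching tutorial text and action map.
; OnActionCompleted compares the reported action with the map entry looked up from the step counter, incrementing on a match.
; One enum value acts as a wildcard that accepts any action, and the event calls itself recursively to auto-advance through it.
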(event Custom|OnActionCompleted
  (params (TakenAction :type Actions%20Enum :default "NewEnumerator0"))
  (bind _output_get (Variables|Default|SetCopyTutorialStep (Variables|Default|GetTutorialStep)))
  (bind _result (Math|Integer|IncrementInt _output_get)
    (:%20%20
      (if (or (Utilities|Enum|Equal(Enum) TakenAction (.Value (Utilities|Map|Find (Variables|Default|GetCurrentActionMap) _result))) (Utilities|Enum|Equal(Enum) (.Value (Utilities|Map|Find (Variables|Default|GetCurrentActionMap) _result)) "NewEnumerator5"))
        (Math|Integer|IncrementInt (Variables|Default|GetTutorialStep)
          (:%20%20
            (bind _result_2 (Math|Integer|IncrementInt (Variables|Default|GetCopyTutorialStep))
              (:%20%20
                (if (Utilities|Enum|Equal(Enum) "NewEnumerator5" (.Value (Utilities|Map|Find (Variables|Default|GetCurrentActionMap) _result_2)))
                  (CallFunction|OnActionCompleted "NewEnumerator5"))))))))))

(event Custom|SetCurrentTutorialMap
  (switch int (Variables|Default|GetCurrentTutorial)
    (:1
      (Variables|Default|SetCurrentTutorialText (Variables|Default|GetTutorialText1))
      (Variables|Default|SetCurrentActionMap (Variables|Default|GetActionMap1)))
    (:2
      (Variables|Default|SetCurrentTutorialText (Variables|Default|GetTutorialText2))
      (Variables|Default|SetCurrentActionMap (Variables|Default|GetActionMap2)))
    (:3
      (Variables|Default|SetCurrentTutorialText (Variables|Default|GetTutorialText3))
      (Variables|Default|SetCurrentActionMap (Variables|Default|GetActionMap3)))
    (:4
      (Variables|Default|SetCurrentTutorialText (Variables|Default|GetTutorialText4))
      (Variables|Default|SetCurrentActionMap (Variables|Default|GetActionMap4)))
    (:5
      (Variables|Default|SetCurrentTutorialText (Variables|Default|GetTutorialText5))
      (Variables|Default|SetCurrentActionMap (Variables|Default|GetActionMap5)))
    (:6
      (Variables|Default|SetCurrentTutorialText (Variables|Default|GetTutorialText6))
      (Variables|Default|SetCurrentActionMap (Variables|Default|GetActionMap6)))))

(fn ConstructionScript)
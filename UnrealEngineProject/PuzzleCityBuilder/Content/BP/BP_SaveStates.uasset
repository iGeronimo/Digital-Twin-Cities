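; BP_SaveStates snapshots and restores the state of a hexagon tile board held in GridTracker.
; Releasing Ctrl+C stores each tile's CurrentTileState in the in-memory SavedGrid array; Ctrl+V writes those states back by index.
; ApplySaveFile applies a supplied TileStates array to the grid the same way.
; A CopyHexagonTileArray helper copies arrays element by element, but nothing in this Blueprint calls it.
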(event Custom|Apply%20Save%20File
  (params (TileStates :type Array%20of%20TileState%20Enums :default "NewEnumerator0"))
  (for (_array_element _array_index) TileStates
    (Variables|/Game/BP/BP_HexagonTile.BP_HexagonTile_C|SetCurrentTileState (Utilities|Array|Get(acopy) (Variables|Default|GetGridTracker) _array_index) _array_element)))

(event Input|KeyboardEvents|CtrlC
  (params (Key :type Key%20Structure :default "None"))
  ;[1 1 1] Save State
  (:Released
    (Utilities|Array|Clear (Variables|Default|GetSavedGrid))
    (for _array_element (Variables|Default|GetGridTracker)
      (bind _asbp_hexagon_tile (Utilities|Casting|CastToBP_HexagonTile _array_element))
      (Utilities|Array|Add (Variables|Default|GetSavedGrid) (Variables|/Game/BP/BP_HexagonTile.BP_HexagonTile_C|GetCurrentTileState _asbp_hexagon_tile)))
    (Development|PrintString "Saved Current Board")))

(event Input|KeyboardEvents|CtrlV
  (params (Key :type Key%20Structure :default "None"))
  ;[1 1 1] Load State
  (:Released
    (for (_array_element _array_index) (Variables|Default|GetGridTracker)
      (bind _asbp_hexagon_tile (Utilities|Casting|CastToBP_HexagonTile _array_element))
      (Variables|/Game/BP/BP_HexagonTile.BP_HexagonTile_C|SetCurrentTileState _asbp_hexagon_tile (Utilities|Array|Get(acopy) (Variables|Default|GetSavedGrid) _array_index)))
    (Development|PrintString "Loaded Last Saved Board")))

(fn ConstructionScript)

(fn CopyHexagonTileArray
  (params (CopyArray :type Array%20of%20BP%20Hexagon%20Tile%20Object%20References) (PasteArray :type Array%20of%20BP%20Hexagon%20Tile%20Object%20References))
  (for _index (range 0 (Utilities|Array|LastIndex CopyArray))
    (Development|PrintString "Setting Element")
    (Utilities|Array|SetArrayElem PasteArray _index (Utilities|Array|Get(acopy) CopyArray _index) true)))
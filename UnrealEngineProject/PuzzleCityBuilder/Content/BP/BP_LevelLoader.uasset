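; BP_LevelLoader sets up a hexagon-tile level at BeginPlay from a LevelSaveFile stored in the save slot named by LevelToLoad.
; An ordered sequence caches the save, then passes board size to BP_HexagonGrid, tile states to BP_SaveStates and max moves to BP_TurnManager.
; Each target is found with GetActorOfClass, and a failed cast halts only the load step, so the later steps still run.
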(event EventBeginPlay
  (Utilities|FlowControl|Sequence
    (:then_0
      (bind _returnvalue (SaveGame|LoadGamefromSlot (Variables|Default|GetLevelToLoad)))
      (bind _aslevel_save_file (Utilities|Casting|CastToLevelSaveFile _returnvalue))
      (Variables|Default|SetSaveFileData _aslevel_save_file))
    (:then_1
      (bind _returnvalue_2 (Actor|GetActorOfClass "/Game/BP/BP_HexagonGrid.BP_HexagonGrid_C"))
      (Default|CreateGrid _returnvalue_2 (Variables|/Game/BP/LevelSaveFile.LevelSaveFile_C|GetBoardSize (Variables|Default|GetSaveFileData))))
    (:then_2
      (bind _returnvalue_3 (Actor|GetActorOfClass "/Game/BP/BP_SaveStates.BP_SaveStates_C"))
      (Default|ApplySaveFile _returnvalue_3 (Variables|/Game/BP/LevelSaveFile.LevelSaveFile_C|GetTileStates (Variables|Default|GetSaveFileData))))
    (:then_3
      (bind _returnvalue_4 (Actor|GetActorOfClass "/Game/BP/BP_TurnManager.BP_TurnManager_C"))
      (Default|SetLevelMoves _returnvalue_4 (Variables|/Game/BP/LevelSaveFile.LevelSaveFile_C|GetMaxMoves (Variables|Default|GetSaveFileData))))))

(fn ConstructionScript)
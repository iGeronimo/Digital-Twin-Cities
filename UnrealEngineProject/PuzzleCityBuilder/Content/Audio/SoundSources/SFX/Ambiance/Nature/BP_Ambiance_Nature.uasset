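; Nature ambience actor that adds an audio component at BeginPlay and adapts its sound to camera height.
; Each tick, camera Z drives clamped convolution reverb wetness, which rises with height, and master volume, which falls with it.
; A transportation gain parameter is also updated, with height-based math noted for transport volume.
; E and Q are debug keys that switch the population amount parameter between a set level and zero.
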(event EventBeginPlay
  (bind _returnvalue (AddComponent|AddAudioComponent false))
  (bind _output_get (Variables|Default|SetMS_Ambiance _returnvalue)))

(event Collision|EventActorBeginOverlap
  (params (OtherActor :type Actor%20Object%20Reference)))

(event EventTick
  (params (DeltaSeconds :type Float%20%28single-precision%29))
  (bind _returnvalue (Game|GetPlayerController 0))
  (bind _playercameramanager (Variables|/Script/Engine.PlayerController|GetPlayerCameraManager _returnvalue))
  (bind _returnvalue_2 (Camera|GetCameraLocation _playercameramanager))
  (bind _z (Math|Vector|BreakVector _returnvalue_2))
  (bind _returnvalue_3 (* _z 0.01))
  (Utilities|FlowControl|Sequence
    (:then_0
      (Class|SourceEffectConvolutionReverbPreset|SetSettings (Variables|Default|GetReverb) (Utilities|Struct|MakeSourceEffectConvolutionReverbSettings (Math|Float|Clamp(Float) (- _returnvalue_3 71.0) -96.0 -16.0) -15.0 false)))
    (:then_2
      (Audio|Parameter|SetFloatParameter (stale EventBeginPlay _output_get) "Master_Volume" (Math|Float|Clamp(Float) (- 1.0 (* (- _returnvalue_3 47.0) 0.020625)) 0.2 0.5) :!class /Script/AudioExtensions.AudioParameterControllerInterface))
    (:then_3
      (Audio|Parameter|SetFloatParameter (stale EventBeginPlay _output_get) "Transportation_Gain" (Math|Float|Clamp(Float) (+ (stale _result) 1.0)) :!class /Script/AudioExtensions.AudioParameterControllerInterface))
    (:then_5
      (bind _result (Math|Float|NegateFloat (* _returnvalue_3 0.021277))))))

(event Input|KeyboardEvents|Q
  (params (Key :type Key%20Structure :default "None"))
  (:Pressed
    (bind _output_get (Variables|Default|SetPopulation_Amount 0.0))
    (Audio|Parameter|SetFloatParameter (stale EventBeginPlay _output_get) "Population_Amount" _output_get :!class /Script/AudioExtensions.AudioParameterControllerInterface)))

(event Input|KeyboardEvents|E
  (params (Key :type Key%20Structure :default "None"))
  (:Pressed
    (bind _output_get (Variables|Default|SetPopulation_Amount 2e+01)) ; Population amount debug
    (Audio|Parameter|SetFloatParameter (stale EventBeginPlay _output_get) "Population_Amount" _output_get :!class /Script/AudioExtensions.AudioParameterControllerInterface)))

(fn ConstructionScript)